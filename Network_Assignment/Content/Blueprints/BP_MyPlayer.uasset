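; BP_MyPlayer is a player Blueprint that shows network role, rocket count and health on a WBP_Role widget held by its WidgetRole component.
; On BeginPlay it writes the local net role to the widget as text.
; The OnNumRocketsChanged and OnHealthChanged events push new values into the same widget, so the display updates on change without any Tick logic.
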(event EventBeginPlay
  ;[1 1 1] Event_BeginPlay
  (bind _aswbp_role (Utilities|Casting|CastToWBP_Role (UserInterface|GetUserWidgetObject (Variables|Default|GetWidget_Role))))
  (Default|SetLocalText _aswbp_role (Utilities|Text|ToText(String) (Utilities|String|EnumtoString (Networking|GetLocalRole)))))

(event EventOnHealthChanged
  (params (newHealth :type Float%20%28single-precision%29))
  ;[1 1 1] UpdateHealth
  (bind _aswbp_role (Utilities|Casting|CastToWBP_Role (UserInterface|GetUserWidgetObject (Variables|Default|GetWidget_Role))))
  (Default|SetHealthText _aswbp_role newHealth))

(event EventOnNumRocketsChanged
  (params (newNumRockets :type Integer))
  ;[1 1 1] UpdateNumRockets
  (bind _aswbp_role (Utilities|Casting|CastToWBP_Role (UserInterface|GetUserWidgetObject (Variables|Default|GetWidget_Role))))
  (Default|SetNumRockets _aswbp_role newNumRockets))

(fn ConstructionScript)